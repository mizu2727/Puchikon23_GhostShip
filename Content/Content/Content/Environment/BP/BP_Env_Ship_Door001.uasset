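; Ship door that the player opens, closes and unlocks with a key while standing in its trigger box.
; Box1 overlap binds the door's handler to the player's Recall dispatcher, and leaving clears all bindings on that dispatcher.
; If locked, it spends a key through BPI_PlayerInterface and only unlocks.
; Otherwise it toggles IsOpen with an instant swept quarter-turn rotation and a door sound.
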(event `self.ReceiveBeginPlay`)

(event `self.ReceiveTick`
  (params (DeltaSeconds :type "Float (single-precision)")))

(event `self.Box1.OnComponentBeginOverlap`
  (params (OverlappedComponent :type "PrimitiveComponent Object Reference") (OtherActor :type "Actor Object Reference") (OtherComp :type "PrimitiveComponent Object Reference") (OtherBodyIndex :type Integer) (bFromSweep :type Boolean) (SweepResult :type "HitResult Structure (by ref)"))
  (bind _asbp_player_class (cast `/Game/Originals/BP/BP_PlayerClass` OtherActor))
  (add `/Game/Originals/BP/BP_PlayerClass.Recall` _asbp_player_class (delegate `Recall_イベント`)))

(event `Recall_イベント`
  (bind _returnvalue (`self.K2_GetActorLocation`))
  (bind _asbpi_player_interface (cast `/Game/Originals/BP/BPI_PlayerInterface` (stale `self.Box1.OnComponentBeginOverlap` _asbp_player_class)))
  (if (`self.LockDoor`)
    (bind _returnkeycount (`/Game/Originals/BP/BPI_PlayerInterface.UseKeyCountFunction` _asbpi_player_interface 0))
    (if (> _returnkeycount 0)
      (`/Game/Originals/BP/BPI_PlayerInterface.UseKeyCountFunction` _asbpi_player_interface 1)
      (set `self.LockDoor` false))
    (elif (`self.IsOpen`)
      (`self.K2_AddActorLocalRotation` (struct :`Yaw` -90.0) true)
      (set `self.IsOpen` false)
      (`GameplayStatics.PlaySoundAtLocation` "/Game/Audio/SE/Open_ドア・きしみ04.Open_ドア・きしみ04" _returnvalue (struct) 1.0 1.0 0.0 null null null null)
      (else
        (`self.K2_AddActorLocalRotation` (struct :`Yaw` 90.0) true)
        (set `self.IsOpen` true)
        (`GameplayStatics.PlaySoundAtLocation` "/Game/Audio/SE/Close_ドア・閉める04.Close_ドア・閉める04" _returnvalue (struct) 1.0 1.0 0.0 null null null null)))))

(event `self.Box1.OnComponentEndOverlap`
  (params (OverlappedComponent :type "PrimitiveComponent Object Reference") (OtherActor :type "Actor Object Reference") (OtherComp :type "PrimitiveComponent Object Reference") (OtherBodyIndex :type Integer))
  (bind _asbp_player_class (cast `/Game/Originals/BP/BP_PlayerClass` OtherActor))
  (clear `/Game/Originals/BP/BP_PlayerClass.Recall` _asbp_player_class))

(fn `DoorOpen`)

(fn `UserConstructionScript`)