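; BP_GoalKeyClass is a key pickup actor that grants the player a door key when touched.
; A hit on its Cube component checks whether the other actor is player character 0, casts it to BP_PlayerClass and calls AddKeyCount.
; Any other actor prints a message saying the key cannot be obtained.
; The actor does not destroy or disable itself afterward, so repeated hits can add more keys.
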(event `self.Cube.OnComponentHit`
  (params (HitComponent :type "PrimitiveComponent Object Reference") (OtherActor :type "Actor Object Reference") (OtherComp :type "PrimitiveComponent Object Reference") (NormalImpulse :type "Vector Structure") (Hit :type "HitResult Structure (by ref)"))
  (bind _returnvalue (`GameplayStatics.GetPlayerCharacter` 0))
  ; 扉の鍵を入手する
  (if (== OtherActor _returnvalue)
    (bind _asbp_player_class (cast `/Game/Originals/BP/BP_PlayerClass` _returnvalue))
    (`/Game/Originals/BP/BP_PlayerClass.AddKeyCount` _asbp_player_class)
    (else
      (`KismetSystemLibrary.PrintString` "鍵を入手できません"))))

(fn `UserConstructionScript`
  (`parent.UserConstructionScript`))