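; BP_Enemy is a patrolling enemy that kills the player on sight.
; From BeginPlay it loops through MoveToLocations with AIMoveTo, pausing briefly before each move and advancing only on success.
; Each Tick swings two Eye components in a sine-driven pitch sweep and line-traces along their up vectors, calling PlayerKill on any BP_PlayerClass hit.
; EnemyLocationChangeTime only prints a debug string.
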(event `self.ReceiveBeginPlay`
  (set `self.Eyes` (`|MakeArray` (`self.Eye`) (`self.Eye1`)))
  (`KismetSystemLibrary.Delay` 0.5 :!label _label)
  (`|AIMoveTo` self (`|GetArrayItem` (`self.MoveToLocations`) (`self.MoveToLocationsInt`)) null
    (:`OnSuccess`
      (set `self.MoveToLocationsInt` (mod (+ (`self.MoveToLocationsInt`) 1) (`KismetArrayLibrary.Array_Length` (`self.MoveToLocations`))))
      (goto _label))))

(event `self.ReceiveTick`
  (params (DeltaSeconds :type "Float (single-precision)"))
  (set `self.RaycastMove` (+ (`self.RaycastMove`) (* DeltaSeconds 1000.0)))
  (set `self.RaycastMove` (mod (`self.RaycastMove`) (* (`KismetMathLibrary.GetPI`) 1000.0)))
  (for _array_element (`self.Eyes`)
    (`SceneComponent.K2_SetRelativeRotation` _array_element (`KismetMathLibrary.MakeRotator` -10.0 (* (`KismetMathLibrary.DegSin` (`self.RaycastMove`)) 40.0)) false false)
    (bind _returnvalue (`SceneComponent.K2_GetComponentLocation` _array_element))
    (bind _outhit (`KismetSystemLibrary.LineTraceSingle` _returnvalue (+ (* (`KismetMathLibrary.TransformDirection` (`SceneComponent.K2_GetComponentToWorld` _array_element) (`KismetMathLibrary.MakeVector` 0.0 0.0 1.0)) (`self.EnemyRaycastScale`)) _returnvalue) "TraceTypeQuery1" true))
    (bind _asbp_player_class (cast `/Game/Originals/BP/BP_PlayerClass` (`.HitActor` (`GameplayStatics.BreakHitResult` _outhit))))
    (`/Game/Originals/BP/BP_PlayerClass.PlayerKill` _asbp_player_class)))

(fn `EnemyLocationChangeTime`
  (`KismetSystemLibrary.PrintString` "Location"))

(fn `UserConstructionScript`)